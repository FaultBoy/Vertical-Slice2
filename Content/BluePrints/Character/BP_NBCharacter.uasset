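; BP_NBCharacter is a character Blueprint with weapon attachment, noise emission and simple contact damage.
; On BeginPlay it caches the BP_PlayController and plays a one-shot shoot-pose animation on the mesh.
; AttachEquipmenttoHand snaps the current weapon to the hand socket and shows it.
; The N key emits noise through the pawn noise emitter with an audible cue, and capsule overlap with a SkinnyMonster decrements health.
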(event OnComponentBeginOverlap(CapsuleComponent)
  (params (OverlappedComponent :type Primitive%20Component%20Object%20Reference) (OtherActor :type Actor%20Object%20Reference) (OtherComp :type Primitive%20Component%20Object%20Reference) (OtherBodyIndex :type Integer) (bFromSweep :type Boolean) (SweepResult :type Hit%20Result%20Structure%20%28by%20ref%29))
  (Utilities|Casting|CastToSkinnyMonster OtherActor)
  (bind _result (Math|Float|DecrementFloat (Variables|Default|GetCurrentHealth))
    (:%20%20
      (Variables|Default|SetCurrentHealth _result)
      (Development|PrintString "" true true "(R=0.235314,G=0.334807,B=1.000000,A=1.000000)"))))

(event EventBeginPlay
  (bind _asbp_play_controller (Utilities|Casting|CastToBP_PlayController (Game|GetPlayerController 0)))
  (Variables|Default|SetPlayerController _asbp_play_controller)
  (Components|Animation|PlayAnimation (Variables|Character|GetMesh) "/Game/Assets/ThirdPerson/Character/Ye/Ye_SkeletalShootPose_Anim.Ye_SkeletalShootPose_Anim" false))

(event Collision|EventActorBeginOverlap
  (params (OtherActor :type Actor%20Object%20Reference)))

(event EventAttachEquipmenttoHand
  (Transformation|AttachComponentToComponent (Variables|Default|GetCurrentWeapon) (Variables|Character|GetMesh) (Class|NBCharacter|GetInventoryAttachPoint "Hands") "SnapToTarget" "SnapToTarget" "SnapToTarget" true)
  (Rendering|SetVisibility (Variables|/Script/No_Bark_Vs.BaseWeapon|GetWeaponMesh (Variables|Default|GetCurrentWeapon)) true false)
  (Development|PrintString "Weapon Spawned"))

(event Input|KeyboardEvents|N
  (params (Key :type Key%20Structure :default "AnyKey"))
  (bind _returnvalue (Transformation|GetActorLocation))
  (:Pressed
    (Class|PawnNoiseEmitterComponent|MakeNoise (Variables|Default|GetPawnNoiseEmitterComp) 0 1.0 _returnvalue)
    (Audio|PlaySoundatLocation "/Engine/EditorSounds/GamePreview/EndPlayInEditor_Cue.EndPlayInEditor_Cue" _returnvalue)))

(fn ConstructionScript)